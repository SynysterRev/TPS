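; Pistol weapon Blueprint that adds metal impact decals where its shots hit.
; Its hit event stores the location and normal, then creates a dynamic instance of the metal decal material with a randomly chosen frame for variation.
; It spawns a small, short-lived decal aligned into the surface from the inverted normal, with random roll so repeated impacts look different.
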(event `self.OnProjectHitEvent`
  (params (HitLocation :type "Vector Structure") (ImpactNormal :type "Vector Structure"))
  (set `self.Hit Location` HitLocation)
  (set `self.Impact Normal` ImpactNormal)
  (bind _returnvalue (`KismetMaterialLibrary.CreateDynamicMaterialInstance` "/Game/BallisticsVFX/Decals/Decals_Metal.Decals_Metal"))
  (bind _output_get (set `self.ImpactDecalMat` _returnvalue))
  (`/Engine/EditorBlueprintResources/StandardMacros.IsValid` _output_get
    (:`Is Valid`
      (`MaterialInstanceDynamic.SetScalarParameterValue` _returnvalue "Frame" (`KismetMathLibrary.Conv_IntToDouble` (`KismetMathLibrary.RandomIntegerInRange` 0 3))))
    (:`Is Not Valid`
      _))
  (`GameplayStatics.SpawnDecalAtLocation` (`self.ImpactDecalMat`) (3.0 3.0 3.0) (`self.Hit Location`) (`KismetMathLibrary.MakeRotator` (`KismetMathLibrary.RandomFloatInRange` 0.0 360.0) (.pitch (`KismetMathLibrary.Conv_VectorToRotator` (* (`self.Impact Normal`) -1))) (.yaw (`KismetMathLibrary.Conv_VectorToRotator` (* (`self.Impact Normal`) -1)))) 10.0))

(fn `UserConstructionScript`)